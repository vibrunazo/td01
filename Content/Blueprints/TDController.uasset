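; Player controller for what appears to be a tower defense game, placing a Tower actor where the player clicks or taps.
; Left click, right click and touch all trace under the cursor on the Visibility channel with complex collision.
; ClickedOnGround stores the hit location, prints it, then spawns the Tower using only its X and Y.
; The hit result is not checked for a blocking hit or surface type before spawning.
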(event `self.ReceiveBeginPlay`)

(event `self.ReceiveTick`
  (params (DeltaSeconds :type "Float (single-precision)")))

(event `Key|LeftMouseButton`
  (params (Key :type "Key Structure" :default "AnyKey"))
  (:`Pressed`
    (`self.ClickedOnGround` (`self.GetHitResultUnderCursorByChannel` "TraceTypeQuery1") :!label _label)))

(event `Key|RightMouseButton`
  (params (Key :type "Key Structure" :default "AnyKey"))
  (:`Pressed`
    (goto _label)))

(event `InputTouch`
  (params (Location :type "Vector Structure") (FingerIndex :type "ETouchIndex Enum"))
  (:`Pressed`
    (goto _label)))

(fn `ClickedOnGround`
  (params (Hit :type "HitResult Structure"))
  (bind (_hit_location_x _hit_location_y) (`KismetMathLibrary.BreakVector` (`self.Hit Location`)))
  (`|ExecutionSequence`
    (:`then_0`
      (bind _output_get (set `self.Hit Location` (`.Location` (`GameplayStatics.BreakHitResult` Hit)))))
    (:`then_1`
      (`KismetSystemLibrary.PrintString` (`KismetStringLibrary.Concat_StrStr` "Hit Location: " (`KismetStringLibrary.Conv_VectorToString` _output_get))))
    (:`then_2`
      (`|SpawnActorFromClass` "/Game/Blueprints/Actors/Chars/Towers/Tower.Tower_C" (`KismetMathLibrary.MakeTransform` (`KismetMathLibrary.MakeVector` _hit_location_x _hit_location_y)) "Undefined" "OverrideRootScale"))))

(fn `UserConstructionScript`)